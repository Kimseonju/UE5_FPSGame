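; BP_DialogComponent is an actor component that runs an NPC-style dialog when a player interacts with its owner.
; At BeginPlay it spawns a dedicated AI controller, using a Behavior Tree as the dialog flow engine.
; Interaction opens the dialog widget in UI-only input, starts the tree and passes the widget through the Blackboard.
; The widget's exit callback restores game input, stops the tree logic and removes the widget.
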(event Custom|OnExit_이벤트_0
  (bind _dialogwidget (Variables|Default|GetDialogWidget))
  (bind _returnvalue (Widget|GetOwningPlayer _dialogwidget))
  (Input|SetInputModeGameOnly _returnvalue)
  (Variables|/Script/Engine.PlayerController|SetbShowMouseCursor _returnvalue false)
  (AI|Logic|StopLogic (Variables|/Script/AIModule.AIController|GetBrainComponent (Variables|Default|GetAIController)) "DialogExited")
  (Widget|RemovefromParent (Variables|Default|GetDialogWidget)))

(event EventBeginPlay
  (bind _returnvalue (Game|SpawnActorfromClass "/Game/Blueprints/DialogSystem/DialogAIController.DialogAIController_C" (Math|Transform|MakeTransform "0, 0, 0" "0, 0, 0" "1.000000,1.000000,1.000000") "Undefined" 0 0))
  (bind _output_get (Variables|Default|SetAIController _returnvalue))
  (Actor|SetOwner _output_get (Components|GetOwner)))

(event EventTick
  (params (DeltaSeconds :type Float%20%28single-precision%29)))

(event EventOnInteraction
  (params (PlayerCharacter :type BP%20Multi%20Play%20Character%201%20Object%20Reference))
  (bind _aicontroller (Variables|Default|GetAIController))
  (bind _as플레이어_컨트롤러 (Utilities|Casting|CastToPlayerController (Pawn|GetController PlayerCharacter)))
  (bind _returnvalue (UserInterface|CreateWidget "/Game/Blueprints/DialogSystem/DialogWidget.DialogWidget_C" _as플레이어_컨트롤러))
  (bind _output_get (Variables|Default|SetDialogWidget _returnvalue))
  (EventDispatchers|AssignOnExit _output_get (delegate Custom|OnExit_이벤트_0))
  (UserInterface|Viewport|AddtoViewport _output_get 0)
  (Input|SetInputModeUIOnly _as플레이어_컨트롤러 _output_get "DoNotLock")
  (Variables|/Script/Engine.PlayerController|SetbShowMouseCursor _as플레이어_컨트롤러 true)
  (AI|RunBehaviorTree _aicontroller (Variables|Default|GetDialogTree))
  (bind _blackboardcomponent (Class|AIController|UseBlackboard _aicontroller "/Game/Blueprints/DialogSystem/DialogBlackboard.DialogBlackboard"))
  (AI|Components|Blackboard|SetValueasObject _blackboardcomponent (Utilities|Name|MakeLiteralName "DialogWidget") (Variables|Default|GetDialogWidget)))