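; BP_ProjectGrenade is a grenade projectile Blueprint that applies Chaos physics fields when destroyed, to break and scatter destructible geometry.
; It binds to its own OnDestroyed at BeginPlay and centers the fields on the collision box.
; A radial falloff applies external cluster strain over twice the outer damage radius.
; A radial vector, wrapped in a culling field, then applies outward linear velocity.
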(event Custom|OnDestroyed_이벤트_0
  (params (DestroyedActor :type Actor%20Object%20Reference))
  (bind _fieldsystemcomponent (Variables|Default|GetFieldSystemComponent))
  (bind _collisionbox (Variables|Default|GetCollisionBox))
  (bind _returnvalue (Transformation|GetWorldLocation _collisionbox))
  (Class|FieldSystemComponent|ApplyPhysicsField _fieldsystemcomponent true "Field_ExternalClusterStrain" 0 (Field|SetRadialFalloff (Variables|Default|GetRadialFalloff) 5e+05 0.0 1.0 0.0 (* (Variables|Default|GetDamageOuterRadius) 2.0) _returnvalue "Field_FallOff_None"))
  (Class|FieldSystemComponent|ApplyPhysicsField _fieldsystemcomponent true "Field_LinearVelocity" 0 (Field|SetCullingField (Variables|Default|GetCullingField) 0 (Field|SetRadialVector (Variables|Default|GetRadialVector) 1e+03 _returnvalue) "Field_Culling_Inside")))

(event EventBeginPlay
  (Game|AssignOnDestroyed (delegate Custom|OnDestroyed_이벤트_0)))

(fn ConstructionScript)