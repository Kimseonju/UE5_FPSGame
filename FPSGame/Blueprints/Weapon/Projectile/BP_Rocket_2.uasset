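; Rocket projectile Blueprint that breaks and pushes Chaos destructible objects around its impact point.
; On a CollisionBox hit, it applies an external cluster strain field from a radial falloff sized by DamageOuterRadius.
; It then applies a linear velocity field from a radial vector centered on the box, passed through an inside culling field.
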(event Custom|OnComponentHit_이벤트_0
  (params (HitComponent :type Primitive%20Component%20Object%20Reference) (OtherActor :type Actor%20Object%20Reference) (OtherComp :type Primitive%20Component%20Object%20Reference) (NormalImpulse :type Vector) (Hit :type Hit%20Result%20Structure%20%28by%20ref%29))
  (bind _fieldsystemcomponent (Variables|Default|GetFieldSystemComponent))
  (bind _collisionbox (Variables|Default|GetCollisionBox))
  (bind _returnvalue (Transformation|GetWorldLocation _collisionbox))
  (Class|FieldSystemComponent|ApplyPhysicsField _fieldsystemcomponent true "Field_ExternalClusterStrain" 0 (Field|SetRadialFalloff (Variables|Default|GetRadialFalloff) 5e+05 0.0 1.0 0.0 (* (Variables|Default|GetDamageOuterRadius) 1.0) _returnvalue "Field_FallOff_None"))
  (Class|FieldSystemComponent|ApplyPhysicsField _fieldsystemcomponent true "Field_LinearVelocity" 0 (Field|SetCullingField (Variables|Default|GetCullingField) 0 (Field|SetRadialVector (Variables|Default|GetRadialVector) 5e+05 _returnvalue) "Field_Culling_Inside")))

(event EventBeginPlay
  (Collision|AssignOnComponentHit (Variables|Default|GetCollisionBox) (delegate Custom|OnComponentHit_이벤트_0)))

(fn ConstructionScript)