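; Quest-reaction wall Blueprint in the NPC folder that breaks a Chaos geometry collection through field system events.
; BoomEvent applies a huge, falloff-free radial external cluster strain centered on ChaosCollectionActor to fracture it.
; BoomEvent2 sends a culled radial vector from the same center, also typed as external cluster strain rather than a force or velocity.
; Nothing in this Blueprint calls either event.
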(event Custom|BoomEvent
  (Class|FieldSystemComponent|ApplyPhysicsField (Variables|Default|GetFieldSystem) true "Field_ExternalClusterStrain" 0 (Field|SetRadialFalloff (Variables|Default|GetRadialFalloff) 5e+08 0.0 1.0 0.0 4e+04 (Transformation|GetActorLocation (Variables|Default|GetChaosCollectionActor)) "Field_FallOff_None")))

(event Custom|BoomEvent2
  (Class|FieldSystemComponent|ApplyPhysicsField (Variables|Default|GetFieldSystem) true "Field_ExternalClusterStrain" 0 (Field|SetCullingField (Variables|Default|GetCullingField) 0 (Field|SetRadialVector (Variables|Default|GetRadialVector) 5e+04 (Transformation|GetActorLocation (Variables|Default|GetChaosCollectionActor))) "Field_Culling_Inside")))

(fn ConstructionScript)