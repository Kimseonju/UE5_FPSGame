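; Basic_Impact is a map-placed destruction actor that breaks Chaos geometry and deals heavy damage within its Sphere component's radius.
; On BeginPlay it applies an external cluster strain field with no falloff through its FieldSystemComponent, plus radial damage, both sized and centered on the sphere.
; FieldEvent calls PlayTo on the LevelSequenceActor found by class lookup, then immediately repeats the same strain and damage.
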(event Custom|FieldEvent
  (bind _sphere (Variables|Default|GetSphere))
  (bind _returnvalue (Transformation|GetWorldLocation _sphere))
  (bind _returnvalue_2 (Components|Sphere|GetScaledSphereRadius _sphere))
  (bind _returnvalue_3 (Actor|GetActorOfClass "/Script/LevelSequence.LevelSequenceActor"))
  (Class|MovieSceneSequencePlayer|Playto (Variables|/Script/LevelSequence.LevelSequenceActor|GetSequencePlayer _returnvalue_3))
  (Class|FieldSystemComponent|ApplyPhysicsField (Variables|Field|GetFieldSystemComponent) true "Field_ExternalClusterStrain" 0 (Field|SetRadialFalloff (Variables|Default|GetRadialFalloff) 5e+05 0.0 1.0 0.0 _returnvalue_2 _returnvalue "Field_FallOff_None"))
  (Game|Damage|ApplyRadialDamage 5e+03 _returnvalue _returnvalue_2 0 0 0 0 false "ECC_Visibility"))

(event EventBeginPlay
  (bind _sphere (Variables|Default|GetSphere))
  (bind _returnvalue (Transformation|GetWorldLocation _sphere))
  (bind _returnvalue_2 (Components|Sphere|GetScaledSphereRadius _sphere))
  (Class|FieldSystemComponent|ApplyPhysicsField (Variables|Field|GetFieldSystemComponent) true "Field_ExternalClusterStrain" 0 (Field|SetRadialFalloff (Variables|Default|GetRadialFalloff) 5e+05 0.0 1.0 0.0 _returnvalue_2 _returnvalue "Field_FallOff_None"))
  (Game|Damage|ApplyRadialDamage 5e+03 _returnvalue _returnvalue_2 0 0 0 0 false "ECC_Visibility"))

(fn ConstructionScript)