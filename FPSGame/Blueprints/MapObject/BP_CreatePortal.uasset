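; BP_CreatePortal is a map object that lays out a spline-based portal with a door at each end.
; Its construction script adds a spline mesh component per segment, using each point's location and tangent to follow the curve.
; It snaps Door1 and BoxCol1 to the first point and Door2 and BoxCol2 to the last, yawed 90 degrees from the spline.
; The event graph holds only empty events, with no teleport or overlap logic.
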(event EventBeginPlay)

(event Collision|EventActorBeginOverlap
  (params (OtherActor :type Actor%20Object%20Reference)))

(event EventTick
  (params (DeltaSeconds :type Float%20%28single-precision%29)))

(fn ConstructionScript
  (bind _spline (Variables|Default|GetSpline))
  (bind _spline_2 (Variables|Default|GetSpline))
  (bind _spline_3 (Variables|Default|GetSpline))
  (bind _returnvalue (Spline|GetTransformatSplinePoint _spline_3 0 "Local" false))
  (bind _returnvalue_2 (Spline|GetNumberOfSplinePoints _spline_2))
  (bind _returnvalue_3 (+ (.yaw (.rotation _returnvalue)) 9e+01))
  (bind _returnvalue_4 (- _returnvalue_2 1))
  (bind _returnvalue_5 (Spline|GetTransformatSplinePoint _spline_2 _returnvalue_4 "Local" false))
  (bind _returnvalue_6 (+ (.yaw (.rotation _returnvalue_5)) 9e+01))
  (for _index (range 0 (- (Spline|GetNumberOfSplinePoints (Variables|Default|GetSpline)) 2))
    (bind _returnvalue_7 (AddComponent|AddSplineMeshComponent false))
    (SplineMesh|SetStartandEnd _returnvalue_7 (.Location (Spline|GetLocationandTangentatSplinePoint _spline _index "Local")) (.Tangent (Spline|GetLocationandTangentatSplinePoint _spline _index "Local")) (.Location (Spline|GetLocationandTangentatSplinePoint _spline (+ _index 1) "Local")) (.Tangent (Spline|GetLocationandTangentatSplinePoint _spline (+ _index 1) "Local")) true :!class /Script/Engine.SplineMeshComponent)
    (Transformation|SetRelativeLocationAndRotation (Variables|Default|GetDoor1) (.location _returnvalue) (Math|Rotator|MakeRotator (.roll (.rotation _returnvalue)) (.pitch (.rotation _returnvalue)) _returnvalue_3) false false)
    (Transformation|SetRelativeLocationAndRotation (Variables|Default|GetBoxCol1) (.location _returnvalue) (Math|Rotator|MakeRotator (.roll (.rotation _returnvalue)) (.pitch (.rotation _returnvalue)) _returnvalue_3) false false)
    (Transformation|SetRelativeLocationAndRotation (Variables|Default|GetDoor2) (.location _returnvalue_5) (Math|Rotator|MakeRotator (.roll (.rotation _returnvalue_5)) (.pitch (.rotation _returnvalue_5)) _returnvalue_6) false false)
    (Transformation|SetRelativeLocationAndRotation (Variables|Default|GetBoxCol2) (.location _returnvalue_5) (Math|Rotator|MakeRotator (.roll (.rotation _returnvalue_5)) (.pitch (.rotation _returnvalue_5)) _returnvalue_6) false false)))