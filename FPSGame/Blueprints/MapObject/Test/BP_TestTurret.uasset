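; Test turret actor that sweeps a laser, acquires players and has hitscan firing logic.
; A looping MoveComponentTo patrols Followtarget between two points, and a traced Niagara beam follows it.
; Cube overlap sets Target after a line-of-sight trace; Tick feeds BeamTarget to the anim blueprint's look-at, though its zero-alpha lerps freeze it.
; Shooting, uncalled here, repeats effects and traces until sight is lost; OnBulletFire is empty.
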(event OnComponentBeginOverlap(Cube)
  (params (OverlappedComponent :type Primitive%20Component%20Object%20Reference) (OtherActor :type Actor%20Object%20Reference) (OtherComp :type Primitive%20Component%20Object%20Reference) (OtherBodyIndex :type Integer) (bFromSweep :type Boolean) (SweepResult :type Hit%20Result%20Structure%20%28by%20ref%29))
  (bind (_outhit _returnvalue) (Collision|LineTraceByChannel (Transformation|GetSocketLocation (Variables|Default|GetTurret) "Circle_002") (Transformation|GetActorLocation OtherActor) "TraceTypeQuery1" false 0 "None"))
  (if _returnvalue
    (if (== OtherActor (.HitActor (Collision|BreakHitResult _outhit)))
      (bind _asmulti_play_character (Utilities|Casting|CastToMultiPlayCharacter OtherActor))
      (Variables|Default|SetTarget _asmulti_play_character)
      (Development|PrintString (Utilities|GetDisplayName (.HitActor (Collision|BreakHitResult _outhit)))))
    (else
      (Variables|Default|SetTarget 0))))

(event Custom|LoopTarget
  (bind _followtarget (Variables|Default|Getfollowtarget))
  (Components|MoveComponentTo _followtarget (Variables|/Script/Engine.SceneComponent|GetRelativeLocation (Variables|Default|Gettarget1)) "0, 0, 0" false false 5.0 false)
  (Components|MoveComponentTo _followtarget (Variables|/Script/Engine.SceneComponent|GetRelativeLocation (Variables|Default|Gettarget2)) "0, 0, 0" false false 5.0 false)
  (CallFunction|LoopTarget))

(event Custom|Event%20Shooting
  (bind _turret (Variables|Default|GetTurret))
  (bind _returnvalue (Transformation|GetSocketLocation _turret "Circle_002"))
  (Utilities|IsValid (Variables|Default|GetTarget) :!label _label
    (:Is%20Valid
      (Components|Activation|Activate (Variables|Default|GetP_AssaultRifle_MuzzleFlash) true)
      (Audio|PlaySoundatLocation "/Game/Assets/Sounds/Ambient/Fire01.Fire01" _returnvalue "0, 0, 0" 1.0 1.0 0.0 0 0 0 0)
      (bind (_outhit _returnvalue_2) (Collision|LineTraceByChannel _returnvalue (Transformation|GetActorLocation (Variables|Default|GetTarget)) "TraceTypeQuery1" false 0 "None"))
      (if _returnvalue_2
        (CallFunction|OnBulletFire)
        (if (== (.HitActor (Collision|BreakHitResult _outhit)) (Variables|Default|GetTarget))
          (Utilities|FlowControl|Delay 0.5)
          (goto _label)
          (else
            _)))
      (Variables|Default|SetTarget 0))))

(event Custom|On%20Bullet%20Fire)

(event EventBeginPlay
  (bind _asbpa_turret (Utilities|Casting|CastToBPA_Turret (Components|SkeletalMesh|GetAnimInstance (Variables|Default|GetTurret))))
  (Variables|Default|SetAs%20BPA%20Turret _asbpa_turret)
  (CallFunction|LoopTarget))

(event Collision|EventActorBeginOverlap
  (params (OtherActor :type Actor%20Object%20Reference)))

(event EventTick
  (params (DeltaSeconds :type Float%20%28single-precision%29))
  (bind _target (Variables|Default|GetTarget))
  (Utilities|IsValid _target
    (:Is%20Valid
      (Variables|Default|SetBeamTarget (Math|Vector|Lerp(Vector) (Variables|Default|GetBeamTarget) (Transformation|GetActorLocation _target) 0.0)))
    (:Is%20Not%20Valid
      (Variables|Default|SetBeamTarget (Math|Vector|Lerp(Vector) (Variables|Default|GetBeamTarget) (Transformation|GetWorldLocation (Variables|Default|Getfollowtarget)) 0.0))))
  (Variables|/Game/Assets/Turret/BPA_Turret.BPA_Turret_C|Setlook%20at%20rotation (Variables|Default|GetAs%20BPA%20Turret) (Math|Rotator|FindLookatRotation (Transformation|GetSocketLocation (Variables|Default|GetTurret) "Circle_002") (Variables|Default|GetBeamTarget)))
  (CallFunction|UpdateLaserBeam))

(fn ConstructionScript)

(fn UpdateLaserBeam
  (bind _followtarget (Variables|Default|Getfollowtarget))
  (bind _laserbeam (Variables|Default|GetLaserBeam))
  (bind _returnvalue (Transformation|GetWorldLocation _followtarget))
  (bind (_outhit _returnvalue_2) (Collision|LineTraceByChannel (Transformation|GetSocketLocation (Variables|Default|GetTurret) "Circle_002") _returnvalue "TraceTypeQuery1" false 0 "None"))
  (if _returnvalue_2
    (Effects|Components|ParticleSystem|SetVectorParameter _laserbeam "User.Beam End" (.Location (Collision|BreakHitResult _outhit)))
    (else
      (Effects|Components|ParticleSystem|SetVectorParameter _laserbeam "User.Beam End" _returnvalue))))