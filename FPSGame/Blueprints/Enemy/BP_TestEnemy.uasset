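; BP_TestEnemy is a test enemy for the FPS game that has a health bar widget and red-tinted mesh materials.
; On BeginPlay it passes itself to its WBP_EnemyHealthBar widget, stopping if the cast fails.
; Dynamic instances of the first four material slots get their EnemyColor set in the Construction Script, then again on BeginPlay with a much lower red intensity.
; Overlap and Tick events are empty.
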(event EventBeginPlay
  (bind _mesh (Variables|Character|GetMesh))
  (bind _aswbp_enemy_health_bar (Utilities|Casting|CastToWBP_EnemyHealthBar (UserInterface|GetUserWidgetObject (Variables|Default|GetHPBarWidget))))
  (Variables|/Game/Blueprints/Widget/WBP_EnemyHealthBar.WBP_EnemyHealthBar_C|SetEnemy _aswbp_enemy_health_bar self)
  (for _index (range 0 3)
    (bind _returnvalue (Rendering|Material|CreateDynamicMaterialInstance _mesh _index (Rendering|Material|GetMaterial _mesh _index) "None" :!class /Script/Engine.PrimitiveComponent))
    (Rendering|Material|SetVectorParameterValue _returnvalue "EnemyColor" (Utilities|Struct|MakeLinearColor 1.0 0.0 0.0 0.0) :!class /Script/Engine.MaterialInstanceDynamic)))

(event Collision|EventActorBeginOverlap
  (params (OtherActor :type Actor%20Object%20Reference)))

(event EventTick
  (params (DeltaSeconds :type Float%20%28single-precision%29)))

(fn ConstructionScript
  (bind _mesh (Variables|Character|GetMesh))
  (for _index (range 0 3)
    (bind _returnvalue (Rendering|Material|CreateDynamicMaterialInstance _mesh _index (Rendering|Material|GetMaterial _mesh _index) "None" :!class /Script/Engine.PrimitiveComponent))
    (Rendering|Material|SetVectorParameterValue _returnvalue "EnemyColor" (Utilities|Struct|MakeLinearColor 1e+01 0.0 0.0 0.0) :!class /Script/Engine.MaterialInstanceDynamic)))