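; Boss enemy Blueprint that fires pooled projectiles at a target and shows a health bar widget.
; BeginPlay hands the boss itself to its WBP_EnemyHealthBar widget.
; Firing, gated on an EnemyAIController, pulls a Projectile from ObjectPoolBullet and launches it at fixed speed along the boss-to-target direction.
; Each spawn point sits ahead of the boss with a random positional offset, so shots scatter on parallel paths.
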(event Custom|Firing
  (params (Target :type Actor%20Object%20Reference))
  (bind _returnvalue (Transformation|GetActorLocation))
  (bind _returnvalue_2 (Transformation|GetActorLocation Target))
  (bind _returnvalue_3 (- _returnvalue_2 _returnvalue))
  (bind _returnvalue_4 (Math|Vector|Normalize _returnvalue_3))
  ;[1 1 1] Firing
  (Utilities|Casting|CastToEnemyAIController (AI|GetAIController self))
  (bind _returnvalue_5 (Class|ObjectPoolComponent|SpawnPoolActor (Variables|Default|GetObjectPoolBullet)))
  (bind _asprojectile (Utilities|Casting|CastToProjectile _returnvalue_5))
  (Transformation|SetActorTransform _asprojectile (Math|Transform|MakeTransform (+ (- (Transformation|GetActorLocation) (Math|Vector|MakeVector (Math|Random|RandomFloatinRange -1.5e+02 1.5e+02) (Math|Random|RandomFloatinRange -1.5e+02 1.5e+02) (Math|Random|RandomFloatinRange -1.5e+02 1.5e+02))) (* _returnvalue_4 2e+02) "") (Math|Conversions|RotationFromXVector _returnvalue_4) "1.000000,1.000000,1.000000"))
  (Actor|SetOwner _asprojectile self)
  (Class|Projectile|SetVelocity _asprojectile _returnvalue_4 1.5e+03))

(event EventBeginPlay
  (bind _aswbp_enemy_health_bar (Utilities|Casting|CastToWBP_EnemyHealthBar (UserInterface|GetUserWidgetObject (Variables|Default|GetHPBarWidget))))
  (Variables|/Game/Blueprints/Widget/WBP_EnemyHealthBar.WBP_EnemyHealthBar_C|SetEnemy _aswbp_enemy_health_bar self))

(fn ConstructionScript)