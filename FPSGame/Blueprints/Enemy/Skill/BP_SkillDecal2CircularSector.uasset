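; BP_SkillDecal2CircularSector is an enemy skill decal actor that shows a circular sector with a timed fill, then removes itself.
; On BeginPlay it creates dynamic materials for the Circum and Area components, using a scalar switch to select outline or area and a shared radian value for the sector.
; After a short delay, a timeline drives the area fill parameter, and the actor destroys itself shortly after it finishes.
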(event EventBeginPlay
  (Utilities|FlowControl|Sequence
    (:then_0
      (bind _returnvalue (Rendering|Material|CreateDynamicMaterialInstance (Variables|Default|GetCircum) :!class /Script/Engine.DecalComponent))
      (bind _output_get (Variables|Default|SetCircumInstance _returnvalue))
      (Rendering|Material|SetScalarParameterValue _output_get "Circum1Area0" 1.0 :!class /Script/Engine.MaterialInstanceDynamic))
    (:then_1
      (bind _returnvalue_2 (Rendering|Material|CreateDynamicMaterialInstance (Variables|Default|GetArea) :!class /Script/Engine.DecalComponent))
      (bind _output_get_2 (Variables|Default|SetAreaInstance _returnvalue_2))
      (Rendering|Material|SetScalarParameterValue _output_get_2 "Circum1Area0" 0.0 :!class /Script/Engine.MaterialInstanceDynamic))
    (:then_2
      (Rendering|Material|SetScalarParameterValue (Variables|Default|GetCircumInstance) "RadianValue" 0.8 :!class /Script/Engine.MaterialInstanceDynamic))
    (:then_3
      (Utilities|FlowControl|Delay 0.2)
      (bind _areavaluealpha (Timeline|타임라인_0 Play)
        (:Update
          (Rendering|Material|SetScalarParameterValue (Variables|Default|GetAreaInstance) "AreaValue" _areavaluealpha :!class /Script/Engine.MaterialInstanceDynamic))
        (:Finished
          (Utilities|FlowControl|Delay 0.2)
          (Actor|DestroyActor))))))

(fn ConstructionScript)