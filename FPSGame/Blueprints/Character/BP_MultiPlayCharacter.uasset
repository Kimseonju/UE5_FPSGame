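; Multiplayer FPS character Blueprint that adds a sniper scope overlay and zipline riding.
; The scope event lazily creates its widget, then plays the zoom animation forward or reversed with matching sounds.
; SetZipline stores the endpoints; jumping while enabled switches to Flying, glides the capsule between them at constant-speed-based duration, then restores Falling.
; Overhead net-role and minimap widget setup are present but disconnected.
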(event EventBeginPlay)

(event Collision|EventActorBeginOverlap
  (params (OtherActor :type Actor%20Object%20Reference)))

(event EventOnJumped
  (bind _startzipline (Variables|Default|GetStartZipline))
  (bind _endzipline (Variables|Default|GetEndZipline))
  (bind _returnvalue (+ _endzipline "0.000000,0,-50.000000"))
  (if (Variables|Default|GetCanZipline)
    (Pawn|Components|CharacterMovement|SetMovementMode (Variables|Character|GetCharacterMovement) "MOVE_Flying" 0)
    (Components|MoveComponentTo (Variables|Default|GetCapsuleComponent) (+ _startzipline "0,0,-50.000000") (Math|Rotator|MakeRotator 0.0 0.0 (.yaw (Math|Rotator|FindLookatRotation _startzipline (Variables|Default|GetEndZipline)))) false false 0.2 false)
    (Components|MoveComponentTo (Variables|Default|GetCapsuleComponent) _returnvalue (Transformation|GetActorRotation) false true (/ (Math|Vector|Distance(Vector) _returnvalue (Variables|Default|GetStartZipline)) 5e+02) false))
  (Pawn|Components|CharacterMovement|SetMovementMode (Variables|Character|GetCharacterMovement) "MOVE_Falling" 0))

(event EventShowSniperScopeWidget
  (params (bShowScape :type Boolean))
  (Utilities|IsValid (Variables|Default|GetSniperScopeWidget)
    (:Is%20Valid
      _)
    (:Is%20Not%20Valid
      (bind _returnvalue (UserInterface|CreateWidget "/Game/Blueprints/Widget/WBP_SniperScape.WBP_SniperScape_C"))
      (bind _output_get (Variables|Default|SetSniperScopeWidget _returnvalue))
      (UserInterface|Viewport|AddtoViewport _output_get 0)))
  (if bShowScape
    (Utilities|IsValid (Variables|Default|GetSniperScopeWidget)
      (:Is%20Valid
        (UserInterface|Animation|PlayAnimation (Variables|Default|GetSniperScopeWidget) (Variables|/Game/Blueprints/Widget/WBP_SniperScape.WBP_SniperScape_C|GetZoomIn (Variables|Default|GetSniperScopeWidget)) 0.0 1 "Forward" 1.0 false)
        (Audio|PlaySound2D "/Game/Assets/MilitaryWeapSilver/Sound/SniperRifle/Cues/SniperRifle_ZoomIn_Cue.SniperRifle_ZoomIn_Cue" 1.0 1.0 0.0 0 0)))
    (else
      (Utilities|IsValid (Variables|Default|GetSniperScopeWidget)
        (:Is%20Valid
          (UserInterface|Animation|PlayAnimation (Variables|Default|GetSniperScopeWidget) (Variables|/Game/Blueprints/Widget/WBP_SniperScape.WBP_SniperScape_C|GetZoomIn (Variables|Default|GetSniperScopeWidget)) 0.0 1 "Reverse" 1.0 false)
          (Audio|PlaySound2D "/Game/Assets/MilitaryWeapSilver/Sound/SniperRifle/Cues/SniperRifle_ZoomOut_Cue.SniperRifle_ZoomOut_Cue" 1.0 1.0 0.0 0 0))))))

(event EventSetZipline
  (params (enable :type Boolean) (Start :type Vector :default "0, 0, 0") (End :type Vector :default "0, 0, 0"))
  (Variables|Default|SetCanZipline enable)
  (Variables|Default|SetStartZipline Start)
  (Variables|Default|SetEndZipline End))

(fn ConstructionScript)