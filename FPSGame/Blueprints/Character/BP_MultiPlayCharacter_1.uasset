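; Player character Blueprint for an FPS, handling interaction, quest UI and sniper scope feedback.
; An overlap sphere tracks InteractionInterface actors or components, and Interact triggers the first in range.
; Tab creates the quest widget, QuestUpdate refreshes it, and the scope event plays zoom animation forward or reversed with sounds.
; Grenade path preview, spline portal travel and net-role display logic is disconnected, leaving ShowProjectilePath and PortalJump empty.
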(event OnComponentBeginOverlap(InteractionSphere)
  (params (OverlappedComponent :type Primitive%20Component%20Object%20Reference) (OtherActor :type Actor%20Object%20Reference) (OtherComp :type Primitive%20Component%20Object%20Reference) (OtherBodyIndex :type Integer) (bFromSweep :type Boolean) (SweepResult :type Hit%20Result%20Structure%20%28by%20ref%29))
  ;[1 1 1] Interact
  (bind _asinteraction_interface (Utilities|Casting|CastToInteractionInterface OtherActor)
    (:then
      (Utilities|Array|AddUnique (Variables|Default|GetInteractablesInRange) _asinteraction_interface))
    (:CastFailed
      (for _array_element (Class|Actor|GetComponentsbyInterface OtherActor "/Game/Blueprints/DialogSystem/InteractionInterface.InteractionInterface_C")
        (Utilities|Array|AddUnique (Variables|Default|GetInteractablesInRange) (.AsInteraction%20Interface (Utilities|Casting|CastToInteractionInterface _array_element)))))))

(event OnComponentEndOverlap(InteractionSphere)
  (params (OverlappedComponent :type Primitive%20Component%20Object%20Reference) (OtherActor :type Actor%20Object%20Reference) (OtherComp :type Primitive%20Component%20Object%20Reference) (OtherBodyIndex :type Integer))
  ;[1 1 1] Interact
  (bind _asinteraction_interface (Utilities|Casting|CastToInteractionInterface OtherActor)
    (:then
      (Utilities|Array|RemoveItem (Variables|Default|GetInteractablesInRange) _asinteraction_interface))
    (:CastFailed
      (for _array_element (Class|Actor|GetComponentsbyInterface OtherActor "/Game/Blueprints/DialogSystem/InteractionInterface.InteractionInterface_C")
        (Utilities|Array|RemoveItem (Variables|Default|GetInteractablesInRange) (.AsInteraction%20Interface (Utilities|Casting|CastToInteractionInterface _array_element)))))))

(event Custom|Show%20Projectile%20Path)

(event Custom|PortalJump
  (params (Spline :type Spline%20Component%20Object%20Reference)))

(event Custom|QuestUpdate
  (bind _questwidget (Variables|Default|GetQuestWidget))
  ;[1 1 1] Quest Test
  (Utilities|IsValid _questwidget
    (:Is%20Valid
      (Default|UpdateQuest _questwidget))))

(event EventTick
  (params (DeltaSeconds :type Float%20%28single-precision%29)))

(event EventShowSniperScopeWidget
  (params (bShowScape :type Boolean))
  (Utilities|IsValid (Variables|Default|GetSniperScopeWidget)
    (:Is%20Valid
      _)
    (:Is%20Not%20Valid
      (bind _returnvalue (UserInterface|CreateWidget "/Game/Blueprints/Widget/WBP_SniperScape.WBP_SniperScape_C"))
      (bind _output_get (Variables|Default|SetSniperScopeWidget _returnvalue))
      (UserInterface|Viewport|AddtoViewport _output_get 0)))
  (if bShowScape
    (Utilities|IsValid (Variables|Default|GetSniperScopeWidget)
      (:Is%20Valid
        (UserInterface|Animation|PlayAnimation (Variables|Default|GetSniperScopeWidget) (Variables|/Game/Blueprints/Widget/WBP_SniperScape.WBP_SniperScape_C|GetZoomIn (Variables|Default|GetSniperScopeWidget)) 0.0 1 "Forward" 1.0 false)
        (Audio|PlaySound2D "/Game/Assets/MilitaryWeapSilver/Sound/SniperRifle/Cues/SniperRifle_ZoomIn_Cue.SniperRifle_ZoomIn_Cue" 1.0 1.0 0.0 0 0)))
    (else
      (Utilities|IsValid (Variables|Default|GetSniperScopeWidget)
        (:Is%20Valid
          (UserInterface|Animation|PlayAnimation (Variables|Default|GetSniperScopeWidget) (Variables|/Game/Blueprints/Widget/WBP_SniperScape.WBP_SniperScape_C|GetZoomIn (Variables|Default|GetSniperScopeWidget)) 0.0 1 "Reverse" 1.0 false)
          (Audio|PlaySound2D "/Game/Assets/MilitaryWeapSilver/Sound/SniperRifle/Cues/SniperRifle_ZoomOut_Cue.SniperRifle_ZoomOut_Cue" 1.0 1.0 0.0 0 0))))))

(event EventBeginPlay
  ;[1 1 1] Quest Test
  (bind _outactors (Actor|GetAllActorsOfClass "/Script/UE5_MultiPlayFPS.Quest"))
  (Variables|Default|SetQuests _outactors))

(event Input|ActionEvents|InputActionInteract
  (params (Key :type Key%20Structure :default "None"))
  ;[1 1 1] Interact
  (:Pressed
    (if (> (Utilities|Array|Length (Variables|Default|GetInteractablesInRange)) 0)
      (Default|OnInteraction (Utilities|Array|Get(acopy) (Variables|Default|GetInteractablesInRange)) self))))

(event Input|KeyboardEvents|Tab
  (params (Key :type Key%20Structure :default "None"))
  ;[1 1 1] Quest Test
  (:Pressed
    (bind _as플레이어_컨트롤러 (Utilities|Casting|CastToPlayerController (Pawn|GetController)))
    (bind _returnvalue (UserInterface|CreateWidget "/Game/Blueprints/Widget/QuestWidget.QuestWidget_C" _as플레이어_컨트롤러))
    (Variables|Default|SetQuestWidget _returnvalue)
    (UserInterface|Viewport|AddtoViewport _returnvalue 0)
    (Widget|SetFocus _returnvalue)))

(fn ConstructionScript)