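; BP_Quest22 is a test quest in the FPSGame quest system that builds its objectives from a set of lights.
; It supplies a TESTBP_QuestObjCollision object as the root objective collection.
; PopulateObjective creates one TESTBP_ObjLight per entry in Lights and adds it to that collection, leaving objective names as None.
; The event graph holds only disabled placeholder events, so the asset's own logic lives in these two construction functions.
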(event EventBeginPlay
  (|CallParentFunction) ; 지금 이 노드는 비활성 상태입니다. \n핀을 끌어서 다른 노드를 연결하면 활성화됩니다.
)

(event Collision|EventActorBeginOverlap
  (params (OtherActor :type Actor%20Object%20Reference)))

(event EventTick
  (params (DeltaSeconds :type Float%20%28single-precision%29)))

(fn ConstructionScript
  (|CallParentFunction))

(fn ConstructRootObjectiveCollection
  (bind _returnvalue (Game|ConstructObjectfromClass self "/Game/Blueprints/QuestSystem/TEST/TESTBP_QuestObjCollision.TESTBP_QuestObjCollision_C" false "None" 0))
  (return _returnvalue))

(fn PopulateObjective
  (params (RootObjCollection :type TESTBP%20Quest%20Obj%20Collision%20Object%20Reference))
  (for _array_element (Variables|Default|GetLights)
    (bind _returnvalue (Game|ConstructObjectfromClass "/Game/Blueprints/QuestSystem/TEST/TESTBP_ObjLight.TESTBP_ObjLight_C" _array_element "None" 0))
    (Default|AddObjective (Variables|Default|GetRootObjectiveCollection) _returnvalue)))