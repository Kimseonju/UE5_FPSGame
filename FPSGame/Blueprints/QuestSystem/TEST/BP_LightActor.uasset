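; BP_LightActor is an interactable light in the quest system's TEST folder that a player switches with the E key while nearby.
; Sphere overlap enables the actor's input for the overlapping BP_MultiPlayCharacter_1's PlayerController and disables it on exit.
; E toggles the PointLight's visibility directly, with no RPC or replication logic in the graph.
; The IsOn? function exposes the light's visibility as its on/off state.
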(event OnComponentBeginOverlap(Sphere)
  (params (OverlappedComponent :type Primitive%20Component%20Object%20Reference) (OtherActor :type Actor%20Object%20Reference) (OtherComp :type Primitive%20Component%20Object%20Reference) (OtherBodyIndex :type Integer) (bFromSweep :type Boolean) (SweepResult :type Hit%20Result%20Structure%20%28by%20ref%29))
  (bind _asbp_multi_play_character_1 (Utilities|Casting|CastToBP_MultiPlayCharacter_1 OtherActor))
  (bind _as플레이어_컨트롤러 (Utilities|Casting|CastToPlayerController (Pawn|GetController _asbp_multi_play_character_1)))
  (Input|EnableInput _as플레이어_컨트롤러))

(event OnComponentEndOverlap(Sphere)
  (params (OverlappedComponent :type Primitive%20Component%20Object%20Reference) (OtherActor :type Actor%20Object%20Reference) (OtherComp :type Primitive%20Component%20Object%20Reference) (OtherBodyIndex :type Integer))
  (bind _asbp_multi_play_character_1 (Utilities|Casting|CastToBP_MultiPlayCharacter_1 OtherActor))
  (bind _as플레이어_컨트롤러 (Utilities|Casting|CastToPlayerController (Pawn|GetController _asbp_multi_play_character_1)))
  (Input|DisableInput _as플레이어_컨트롤러))

(event EventBeginPlay)

(event Collision|EventActorBeginOverlap
  (params (OtherActor :type Actor%20Object%20Reference)))

(event EventTick
  (params (DeltaSeconds :type Float%20%28single-precision%29)))

(event Input|KeyboardEvents|E
  (params (Key :type Key%20Structure :default "None"))
  (:Pressed
    (Rendering|ToggleVisibility (Variables|Default|GetPointLight) false)))

(fn ConstructionScript)

(fn IsOn?
  (return (Variables|/Script/Engine.SceneComponent|GetbVisible (Variables|Default|GetPointLight))))